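; Score Attack Endless mode logic that runs a timed session and ends it once elapsed time exceeds a limit.
; A looping one-second timer, started by StartTimer, counts Time up despite its Removetimer event name.
; While GameStarted is set, Tick shows the controller's HUD and checks the limit.
; GameOver pauses the timer, hides the HUD, saves the point multiplier to the DataGlobal game instance and shows the end HUD.
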(event Custom|StartTimer
  (bind _returnvalue (Utilities|Time|SetTimerbyEvent (delegate Custom|removetimer) 1.0 true)))

(event Custom|removetimer
  (Math|Integer|IncrementInt (Variables|Default|GetTime)))

(event Custom|GameOver
  (Utilities|Time|PauseTimerbyHandle (stale Custom|StartTimer _returnvalue))
  (Widget|SetVisibility (Variables|/Game/Blueprints/ScoreAttackController.ScoreAttackController_C|GetScoreAttackHUD (stale EventTick _asscore_attack_controller)) "Hidden")
  (bind _asscore_attack_controller (Utilities|Casting|CastToScoreAttackController (Game|GetPlayerController 0)))
  (bind _asdata_global (Utilities|Casting|CastToDataGlobal (Game|GetGameInstance))
    (:then
      (Variables|/Game/Blueprints/DataGlobal.DataGlobal_C|SetMultiplier _asdata_global (Variables|/Game/Blueprints/UI/ClickAndDragHUD.ClickAndDragHUD_C|GetPointMultiplier (Variables|/Game/Blueprints/ScoreAttackController.ScoreAttackController_C|GetScoreAttackHUD _asscore_attack_controller)))
      (Widget|SetVisibility (Variables|/Game/Blueprints/ScoreAttackController.ScoreAttackController_C|GetEndHUD _asscore_attack_controller) "Visible")
      (Variables|Default|SetGameStarted? false))
    (:CastFailed
      (Development|PrintString "Hello"))))

(event EventBeginPlay)

(event EventTick
  (params (DeltaSeconds :type Float%20%28single-precision%29))
  (if (Variables|Default|GetGameStarted?)
    (bind _asscore_attack_controller (Utilities|Casting|CastToScoreAttackController (Game|GetPlayerController 0)))
    (Widget|SetVisibility (Variables|/Game/Blueprints/ScoreAttackController.ScoreAttackController_C|GetScoreAttackHUD _asscore_attack_controller) "Visible")
    (if (> (Variables|Default|GetTime) (Variables|Default|GetTimeLimit))
      (CallFunction|GameOver))))

(fn ConstructionScript)