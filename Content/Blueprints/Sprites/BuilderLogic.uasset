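; BuilderLogic is a 2D sprite character that walks back and forth along the X axis and tracks mouse clicks on itself.
; Every tick it adds movement input and yaws the flipbook to match IsMovingLeft, which flips whenever the capsule hits something.
; Pressing and releasing on the capsule sets and clears IsClicked, with presses gated by CanBeClicked.
; Overlapping any TriggerBox turns CanBeClicked off.
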(event OnComponentHit(CapsuleComponent)
  (params (OtherActor :type Actor%20Object%20Reference) (OtherComp :type Primitive%20Component%20Object%20Reference) (NormalImpulse :type Vector :default "0, 0, 0") (Hit :type Hit%20Result%20Structure%20%28by%20ref%29))
  (Variables|Default|SetIsMovingLeft (not (Variables|Default|GetIsMovingLeft))))

(event OnClicked(CapsuleComponent)
  (params (TouchedComponent :type Primitive%20Component%20Object%20Reference))
  (if (Variables|Default|GetCanBeClicked)
    (Variables|Default|SetIsClicked true)))

(event OnReleased(CapsuleComponent)
  (params (TouchedComponent :type Primitive%20Component%20Object%20Reference))
  (Variables|Default|SetIsClicked false))

(event OnComponentBeginOverlap(CapsuleComponent)
  (params (OtherActor :type Actor%20Object%20Reference) (OtherComp :type Primitive%20Component%20Object%20Reference) (OtherBodyIndex :type Integer) (bFromSweep :type Boolean) (SweepResult :type Hit%20Result%20Structure%20%28by%20ref%29))
  (bind _outactors (Actor|GetAllActorsOfClass "/Script/Engine.TriggerBox"))
  (for _array_element _outactors
    (if (== _array_element OtherActor)
      (Variables|Default|SetCanBeClicked false))))

(event Custom|Direction
  (Transformation|SetRelativeRotation (Variables|Default|GetPaperFlipbook) (Math|Rotator|MakeRotator 0.0 0.0 (Math|Float|SelectFloat 0.0 1.8e+02 (Variables|Default|GetIsMovingLeft))) false false)
  (Pawn|Input|AddMovementInput (Math|Vector|SelectVector "1.000000,0.000000, 0" "-1.000000,0.000000, 0" (Variables|Default|GetIsMovingLeft)) 1.0 false))

(event EventTick
  (params (DeltaSeconds :type Float%20%28single-precision%29))
  (CallFunction|Direction))

(fn ConstructionScript)