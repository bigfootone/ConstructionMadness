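; Player controller for the Score Attack click-and-drag mode, letting the player grab and move objects with the mouse.
; BeginPlay creates the start, gameplay and next-gamemode widgets, with the latter two hidden.
; Once ScoreAttackEndless flags the game started, left click traces from the cursor and stores the hit actor.
; While held, Tick sweeps that actor to the deprojected cursor position, locking Y to a fixed plane.
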(event EventBeginPlay
  (bind _returnvalue (UserInterface|CreateWidget "/Game/Blueprints/UI/DragGameStart.DragGameStart_C" (Game|GetPlayerController 0)))
  (bind _output_get (Variables|Default|SetStartWidget _returnvalue))
  (UserInterface|Viewport|AddtoViewport _output_get 0)
  (bind _returnvalue_2 (UserInterface|CreateWidget "/Game/Blueprints/UI/ClickAndDragHUD.ClickAndDragHUD_C" (Game|GetPlayerController 0)))
  (bind _output_get_2 (Variables|Default|SetScoreAttackHUD _returnvalue_2))
  (UserInterface|Viewport|AddtoViewport _output_get_2 0)
  (Widget|SetVisibility _output_get_2 "Hidden")
  (bind _returnvalue_3 (UserInterface|CreateWidget "/Game/Blueprints/UI/MoveToNextGamemodeHUD.MoveToNextGamemodeHUD_C" (Game|GetPlayerController 0)))
  (bind _output_get_3 (Variables|Default|SetEndHUD _returnvalue_3))
  (UserInterface|Viewport|AddtoViewport _output_get_3 0)
  (Widget|SetVisibility _output_get_3 "Hidden"))

(event EventTick
  (params (DeltaSeconds :type Float%20%28single-precision%29))
  (bind (_worldlocation _worlddirection) (Game|Player|ConvertMouseLocationToWorldSpace))
  (bind _returnvalue (* _worlddirection 5e+02))
  (bind _returnvalue_2 (+ _worldlocation _returnvalue))
  (bind (_x _y _z) (Math|Vector|BreakVector _returnvalue_2))
  (bind _asscore_attack_endless (Utilities|Casting|CastToScoreAttackEndless (Game|GetGameMode)))
  (if (Variables|/Game/Blueprints/ScoreAttackEndless.ScoreAttackEndless_C|GetGameStarted? _asscore_attack_endless)
    (if (Variables|Default|GetMouseDown)
      (if (Variables|Default|GetBuilderGrabbed)
        (Transformation|SetActorLocation (Variables|Default|GetObjectGrabbed) (Math|Vector|MakeVector _x 9e+01 _z) true false)))))

(event Input|MouseEvents|LeftMouseButton
  (params (Key :type Key%20Structure :default "AnyKey"))
  (bind (_worldlocation _worlddirection) (Game|Player|ConvertMouseLocationToWorldSpace))
  (:Pressed
    (bind _asscore_attack_endless (Utilities|Casting|CastToScoreAttackEndless (Game|GetGameMode)))
    (if (Variables|/Game/Blueprints/ScoreAttackEndless.ScoreAttackEndless_C|GetGameStarted? _asscore_attack_endless)
      (Variables|Default|SetMouseDown true)
      (bind (_outhit _returnvalue) (Collision|LineTraceByChannel _worldlocation (+ _worlddirection (* _worlddirection 1e+04)) "TraceTypeQuery1" false 0 "None"))
      (if _returnvalue
        (Variables|Default|SetObjectGrabbed (.HitActor (Collision|BreakHitResult _outhit)))
        (Variables|Default|SetBuilderGrabbed true))))
  (:Released
    (bind _asscore_attack_endless_2 (Utilities|Casting|CastToScoreAttackEndless (Game|GetGameMode)))
    (if (Variables|/Game/Blueprints/ScoreAttackEndless.ScoreAttackEndless_C|GetGameStarted? _asscore_attack_endless_2)
      (Variables|Default|SetMouseDown false)
      (Variables|Default|SetBuilderGrabbed false))))

(fn ConstructionScript)